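; BP_Point is a point actor whose Cube mesh shows its state through material swaps.
; The construction script and the IsBlack RepNotify both apply BasicAsset03 when IsBlack is set, with no revert when it clears.
; A second RepNotify on the Event enum colors the cube red for Ship and blue for Event, so state changes reach clients through replication.
; The event graph holds no active logic.
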(event `self.ReceiveBeginPlay`)

(fn `OnRep_event`
  (switch `/Game/Blueprints/E_EventType` (`self.event`)
    (:`NewEnumerator0`
      (`PrimitiveComponent.SetMaterial` (`self.Cube`) 0 "/AnimationSharing/AnimSharingRed.AnimSharingRed"))
    (:`NewEnumerator1`
      (`PrimitiveComponent.SetMaterial` (`self.Cube`) 0 "/AnimationSharing/AnimSharingBlue.AnimSharingBlue"))))

(fn `OnRep_isBlack`
  (if (`self.isBlack`)
    (`PrimitiveComponent.SetMaterial` (`self.Cube`) 0 "/Engine/MapTemplates/Materials/BasicAsset03.BasicAsset03")))

(fn `UserConstructionScript`
  (if (`self.isBlack`)
    (`PrimitiveComponent.SetMaterial` (`self.Cube`) 0 "/Engine/MapTemplates/Materials/BasicAsset03.BasicAsset03")))