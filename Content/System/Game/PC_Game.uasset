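; PC_Game is the player controller for a turn-based dice game, creating the UI_Game widget on BeginPlay.
; Its dice event stores a random six-sided roll on PS_Player, clears that player's turn flag and tells the game state to advance the turn.
; Other events forward lane choices by name to the game state and have the first BP_Camera found set itself up for this controller.
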(event `self.ReceiveBeginPlay`
  (bind _returnvalue (`|CreateWidget` "/Game/UI/UI_Game.UI_Game_C"))
  (`UserWidget.AddToViewport` _returnvalue 0))

(event `lauchDice`
  (bind _asps_player (cast `/Game/Blueprints/PS_Player` (`self.PlayerState`)))
  (set `/Game/Blueprints/PS_Player.DiceLaunch` (`KismetMathLibrary.RandomIntegerInRange` 1 6) _asps_player)
  (set `/Game/Blueprints/PS_Player.isTurn` false _asps_player)
  (`/Game/System/Game/GS_Game.setNextTurn` (`/Game/System/BP_Library.castToGsGame`)))

(event `chooseLine`
  (params (name :type String))
  (`/Game/System/Game/GS_Game.choosingLane` (`/Game/System/BP_Library.castToGsGame`) name))

(event `startingCamera`
  (bind _outactors (`GameplayStatics.GetAllActorsOfClass` "/Game/Blueprints/BP_Camera.BP_Camera_C"))
  (`/Game/Blueprints/BP_Camera.setPlayerCamera` (`|GetArrayItem` _outactors) self))

(fn `UserConstructionScript`)