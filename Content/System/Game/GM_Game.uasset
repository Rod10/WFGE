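; Game mode for the match that builds the two-lane board (A and B) and tracks connected players.
; On BeginPlay it spawns a row of BP_Point actors per lane from EventsLanes and ShipsLane data, tinting ship and event points and storing each row in Lanes.
; Joins and logouts maintain PlayersControllers, with joins also updating player state in the game state.
; Disconnected backup graphs for camera start, session kicking and Lane B never run.
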(event `createPoint`
  (params (tansform :type "Transform Structure") (isBlack :type Boolean) (event :type "/Game/Blueprints/E_EventType Enum" :default "NewEnumerator2") (eventName :type String) (ship :type "/Game/Blueprints/S_Ship Structure"))
  ;[1 1 1] Point Creation
  (bind _returnvalue (`|SpawnActorFromClass` "/Game/Blueprints/BP_Point.BP_Point_C" tansform "AdjustIfPossibleButAlwaysSpawn" "MultiplyWithRoot" null isBlack event eventName 0 ship null))
  (switch `/Game/Blueprints/E_EventType` event
    (:`NewEnumerator2`
      _)
    (:`NewEnumerator0`
      (bind _cube (`/Game/Blueprints/BP_Point.Cube` _returnvalue))
      (`PrimitiveComponent.SetMaterial` _cube 0 "/AnimationSharing/AnimSharingRed.AnimSharingRed"))
    (:`NewEnumerator1`
      (`PrimitiveComponent.SetMaterial` _cube 0 "/AnimationSharing/AnimSharingBlue.AnimSharingBlue")))
  (`KismetArrayLibrary.Array_Add` (`self.Points`) _returnvalue))

(event `createLaneA`
  ;[1 1 1] Lane A Creation
  (`KismetArrayLibrary.Array_Clear` (`self.Points`))
  (for _index (range 76)
    (bind (_type _eventname _color _number) (break `/Game/Blueprints/S_Event` (`|GetArrayItem` (`.eventsLaneA_10_4CB5055B488F24DA2EB9C8BB3044C7A0` (break `/Game/Blueprints/S_EventLane` (`self.EventsLanes`))) _index)))
    (switch `/Game/Blueprints/E_EventType` _type
      (:`NewEnumerator2`
        (bind _returnvalue (`KismetMathLibrary.MakeTransform` (`KismetMathLibrary.MakeVector` 0.0 (`KismetMathLibrary.Conv_IntToDouble` (* _index 200)))))
        (`self.createPoint` _returnvalue))
      (:`NewEnumerator0`
        (`self.createPoint` _returnvalue false "NewEnumerator0" "" (`|GetArrayItem` (`.ShipsLaneA_7_0D9D62544AA3B83293D668A907C208DA` (break `/Game/Blueprints/S_Ships` (`self.ShipsLane`))) _number)))
      (:`NewEnumerator1`
        (`self.createPoint` _returnvalue false "NewEnumerator1" _eventname))))
  (`KismetArrayLibrary.Array_Add` (`self.Lanes`) (make `/Game/Blueprints/S_Lane` "A" (`KismetMathLibrary.Conv_LinearColorToColor` (`KismetMathLibrary.MakeColor` 0.0)) (`self.Points`))))

(event `createLaneB`
  ;[1 1 1] Lane B Creation
  (`KismetArrayLibrary.Array_Clear` (`self.Points`))
  (for _index (range 76)
    (bind (_type _eventname _color _number) (break `/Game/Blueprints/S_Event` (`|GetArrayItem` (`.eventsLaneB_14_56E0360D4581DB6EE664EBB5E1DBC724` (break `/Game/Blueprints/S_EventLane` (`self.EventsLanes`))) _index)))
    (switch `/Game/Blueprints/E_EventType` _type
      (:`NewEnumerator2`
        (bind _returnvalue (`KismetMathLibrary.MakeTransform` (`KismetMathLibrary.MakeVector` -200.0 (`KismetMathLibrary.Conv_IntToDouble` (* _index 200)))))
        (`self.createPoint` _returnvalue true))
      (:`NewEnumerator0`
        (`self.createPoint` _returnvalue true "NewEnumerator0" "" (`|GetArrayItem` (`.ShipLaneB_12_A93BAB354071B376DB2BE4B344070716` (break `/Game/Blueprints/S_Ships` (`self.ShipsLane`))) _number)))
      (:`NewEnumerator1`
        (`self.createPoint` _returnvalue true "NewEnumerator1" _eventname))))
  (`KismetArrayLibrary.Array_Add` (`self.Lanes`) (make `/Game/Blueprints/S_Lane` "B" (`KismetMathLibrary.Conv_LinearColorToColor` (`KismetMathLibrary.MakeColor` 0.0)) (`self.Points`))))

(event `self.ReceiveBeginPlay`
  (`/Engine/EditorBlueprintResources/StandardMacros.DoOnce` false
    (:`Completed`
      (`self.createLaneA`)
      (`self.createLaneB`))))

(event `self.HandleStartingNewPlayer`
  (params (NewPlayer :type "PlayerController Object Reference"))
  (`KismetArrayLibrary.Array_AddUnique` (`self.PlayersControllers`) NewPlayer)
  (`/Game/System/Game/GS_Game.updatePlayerState` (`/Game/System/BP_Library.castToGsGame`)))

(event `self.K2_OnLogout`
  (params (ExitingController :type "Controller Object Reference"))
  (bind _asplayer_controller (cast `PlayerController` ExitingController))
  (`KismetArrayLibrary.Array_RemoveItem` (`self.PlayersControllers`) _asplayer_controller))

(fn `findPlayerIndex`
  (params (player :type "/Game/System/Game/PC_Game Object Reference"))
  (returns (ReturnValue :type Integer))
  (for (_array_element _array_index) (`self.PlayersControllers`)
    (if (== (`Controller.PlayerState` _array_element) (`Controller.PlayerState` player))
      (return _array_index))))

(fn `UserConstructionScript`)