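; GM_Lobby is the lobby game mode that tracks connected players and moves the server to the Game map.
; Login and logout events maintain the PlayersControllers array and trigger a short-delayed player list refresh on the lobby game state.
; launchGame reads the session settings, reapplies them through UpdateSession, then runs a delayed serverTravel console command.
; An unconnected backup branch kicks players beyond the connection limit before travelling.
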(event `self.ReceiveBeginPlay`)

(event `updatePlayerList`
  (`KismetSystemLibrary.Delay` 0.3)
  (`/Game/System/Lobby/GS_Lobby.updatePlayerList` (`/Game/System/BP_Library.castToGSLobby`)))

(event `launchGame`
  (bind (_numconnections _numprivateconnections _bislan _bisdedicated _ballowinvites _ballowjoininprogress _bisanticheatenabled _builduniqueid _extrasettings) (`AdvancedSessionsLibrary.GetSessionSettings`)
    (:`OnSuccess`
      (`UpdateSessionCallbackProxyAdvanced.UpdateSession` _extrasettings _numconnections
        (:`OnSuccess`
          (`KismetSystemLibrary.Delay` 1.0)
          (`KismetSystemLibrary.ExecuteConsoleCommand` "serverTravel Game" null))))))

(event `self.K2_PostLogin`
  (params (NewPlayer :type "PlayerController Object Reference"))
  (`KismetArrayLibrary.Array_AddUnique` (`self.PlayersControllers`) NewPlayer)
  (`self.updatePlayerList`))

(event `self.K2_OnLogout`
  (params (ExitingController :type "Controller Object Reference"))
  (bind _asplayer_controller (cast `PlayerController` ExitingController))
  (`KismetArrayLibrary.Array_RemoveItem` (`self.PlayersControllers`) _asplayer_controller)
  (`self.updatePlayerList`))

(fn `UserConstructionScript`)