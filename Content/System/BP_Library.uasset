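; Blueprint function library of shortcuts that fetch and cast the project's lobby and gameplay framework objects.
; It returns the lobby and game versions of game mode, game state and player controller, plus the player character.
; Controller and character lookups always use player index 0, and each function stops without returning if its cast fails.
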(fn CasttoGmLobby
  (bind _asgm_lobby (Utilities|Casting|CastToGM_Lobby (Game|GetGameMode (LocalVariables|Get__WorldContext))))
  (return _asgm_lobby))

(fn CasttoPCLobby
  (bind _aspc_lobby (Utilities|Casting|CastToPC_Lobby (Game|GetPlayerController (LocalVariables|Get__WorldContext))))
  (return _aspc_lobby))

(fn CasttoGSLobby
  (bind _asgs_lobby (Utilities|Casting|CastToGS_Lobby (Game|GetGameState)))
  (return _asgs_lobby))

(fn CasttoGsGame
  (bind _asgs_game (Utilities|Casting|CastToGS_Game (Game|GetGameState (LocalVariables|Get__WorldContext))))
  (return _asgs_game))

(fn CasttoPCGame
  (bind _aspc_game (Utilities|Casting|CastToPC_Game (Game|GetPlayerController (LocalVariables|Get__WorldContext))))
  (return _aspc_game))

(fn CasttoCGame
  (bind _asc_player (Utilities|Casting|CastToC_Player (Game|GetPlayerCharacter (LocalVariables|Get__WorldContext))))
  (return _asc_player))

(fn CasttoGMGame
  (bind _asgm_game (Utilities|Casting|CastToGM_Game (Game|GetGameMode (LocalVariables|Get__WorldContext))))
  (return _asgm_game))